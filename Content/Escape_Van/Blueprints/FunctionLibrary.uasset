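; Blueprint function library for Escape_Van that converts between 2D unit heading vectors and the four cardinal compass directions.
; One function matches a vector within a small tolerance and returns the direction's name, one-letter code and array index, with +Y as North and +X as East.
; The reverse function returns the vector when any one of index, name or letter matches, testing North, East, South, then West.
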(fn ConvertVectorHeadingtoCompassDirection
  (params (Heading :type Vector%202D%20Structure))
  (if (Math|Vector|Equal(Vector) Heading "(X=0.000000,Y=1.000000)" 0.0001)
    (return "North" "N" 0)
    (elif (Math|Vector|Equal(Vector) Heading "(X=1.000000,Y=0.000000)" 0.0001)
      (return "East" "E" 1)
      (elif (Math|Vector|Equal(Vector) Heading "(X=0.000000,Y=-1.000000)" 0.0001)
        (return "South" "S" 2)
        (elif (Math|Vector|Equal(Vector) Heading "(X=-1.000000,Y=0.000000)" 0.0001)
          (return "West" "W" 3))))))

(fn ConvertCompassDirectiontoVectorHeading
  (params (ArrayIndex :type Integer) (Direction :type String) (Dircetion%281Letter%29 :type String))
  (if (Math|Boolean|ORBoolean (== ArrayIndex 0) (Utilities|Enum|Equal(Enum) Direction "North") (Utilities|Enum|Equal(Enum) Dircetion%281Letter%29 "N"))
    (return "(X=0.000000,Y=1.000000)")
    (elif (Math|Boolean|ORBoolean (== ArrayIndex 1) (Utilities|Enum|Equal(Enum) Direction "East") (Utilities|Enum|Equal(Enum) Dircetion%281Letter%29 "E"))
      (return "(X=1.000000,Y=0.000000)")
      (elif (Math|Boolean|ORBoolean (== ArrayIndex 2) (Utilities|Enum|Equal(Enum) Direction "South") (Utilities|Enum|Equal(Enum) Dircetion%281Letter%29 "S"))
        (return "(X=0.000000,Y=-1.000000)")
        (elif (Math|Boolean|ORBoolean (== ArrayIndex 3) (Utilities|Enum|Equal(Enum) Direction "West") (Utilities|Enum|Equal(Enum) Dircetion%281Letter%29 "W"))
          (return "(X=-1.000000,Y=0.000000)"))))))