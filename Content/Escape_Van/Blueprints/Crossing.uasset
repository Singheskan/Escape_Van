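; Crossing actor for Escape Van that represents a junction in the street network, holding street names and distances for the four compass directions.
; On BeginPlay it caches the game mode, then builds a direction-to-street map and a distance array.
; It counts the non-empty streets, flagging exactly two as turn-only, regardless of their directions, and one as an endpoint.
; Debug prints for streets, coordinates and distances are left unconnected.
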(event EventBeginPlay
  (bind _numberofconnections (Variables|Default|GetNumberOfConnections))
  (bind _asgm_escape_van_alpha_1 (Utilities|Casting|CastToGM_Escape_Van_Alpha1 (Game|GetGameMode)))
  (Variables|References|SetGameMode _asgm_escape_van_alpha_1)
  (bind _output_get (Variables|Default|SetConnectedStreets (Utilities|Map|MakeMap "Street N" (Variables|Default|GetStreet_N) "Street E" (Variables|Default|GetStreet_E) "Street S" (Variables|Default|GetStreet_S) "Street W" (Variables|Default|GetStreet_W))))
  (bind _values (Utilities|Map|Values _output_get))
  (Variables|Default|SetDistancesArray (Utilities|Array|MakeArray (Variables|Default|GetDistance_N) (Variables|Default|GetDistance_E) (Variables|Default|GetDistance_S) (Variables|Default|GetDistance_W)))
  (for _array_element _values
    (if (not (Utilities|Array|IsEmpty _array_element))
      (Math|Integer|IncrementInt (Variables|Default|GetNumberOfConnections))))
  (if (== _numberofconnections 2)
    (Variables|Default|SetIsTurnOnly true)
    (elif (== _numberofconnections 1)
      (Variables|Default|SetIsEndpoint true))))

(fn ConstructionScript)