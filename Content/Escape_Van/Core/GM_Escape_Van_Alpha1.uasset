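; Game mode for the Escape Van alpha that runs a repeating timed round built around guessing a police department's encryption key.
; BeginPlay creates and shows the main HUD, then starts a round that picks a random department from the symbol map, looks up its matching key, and resets the HUD.
; Tick counts down the round timer and starts a new round whenever it runs out.
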(event Custom|StartNewRound
  (Variables|Default|SetTimer 3e+01)
  ;[1 1 1] Randomly choose a Departement and find Key
  (bind _output_get (Variables|Default|SetChosenDepartement (Math|Random|RandomIntegerinRange 0 (- (Utilities|Map|Length (.Police-Symbols (Utilities|Struct|BreakStruct_Lists (Variables|Default|GetStructLists)))) 1))))
  (CallFunction|FindCorrectKey _output_get)
  (Default|Reset (Variables|Default|GetHUD_Reference)))

(event EventBeginPlay
  ;[1 1 1] Create HUD
  (bind _returnvalue (UserInterface|CreateWidget "/Game/Escape_Van/HUD/HUD_Alpha1_Main.HUD_Alpha1_Main_C" (Game|GetPlayerController 0)))
  (bind _output_get (Variables|Default|SetHUD_Reference _returnvalue))
  (UserInterface|Viewport|AddtoViewport _output_get 0)
  (CallFunction|StartNewRound))

(event EventTick
  (params (DeltaSeconds :type Float%20%28single-precision%29))
  (bind _output_get (Variables|Default|SetTimer (- (Variables|Default|GetTimer) DeltaSeconds)))
  (if (<= _output_get 0.0)
    (CallFunction|StartNewRound)))

(fn ConstructionScript)

(fn FindCorrectKey
  (params (IndexOfChosenDepartement :type Integer))
  (bind _structlists (Variables|Default|GetStructLists))
  (bind (_police_symbols _police_encryptionkeys) (Utilities|Struct|BreakStruct_Lists _structlists))
  (bind _keys (Utilities|Map|Keys _police_symbols))
  (bind _output_get (Variables|Default|SetCorrectKey (.Value (Utilities|Map|Find _police_encryptionkeys (Utilities|Array|Get(acopy) _keys IndexOfChosenDepartement)))))
  (if (.ReturnValue (Utilities|Map|Find _police_encryptionkeys (Utilities|Array|Get(acopy) _keys IndexOfChosenDepartement)))
    (Development|PrintString (Utilities|String|Append "Departement Enryption Key: " _output_get) false true "(R=0.000000,G=0.660000,B=1.000000,A=1.000000)" 3e+01)
    (else
      (Development|PrintString "ERROR: Departement not found"))))