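; Player controller for Escape Van that tracks the van's position and heading on a coordinate grid of street crossings.
; On BeginPlay it caches the game mode and van pawn, finds the next crossing and starts a round.
; NewRound advances to that crossing, looks up the following one at position plus heading in the game mode's coordinate map, and starts another round if found.
; SpaceBar debug-checks for a crossing at the heading rotated -90 degrees.
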(event Custom|NewRound
  ;[1 1 1] "Arriving at" Debug
  (bind _values (Utilities|Map|Values (Variables|/Game/Escape_Van/Blueprints/Crossing.Crossing_C|GetConnectedStreets (Variables|Default|GetNextCrossing))))
  (Development|PrintString (Utilities|String|Append "Arriving at: " (Utilities|String|JoinStringArray _values " X ")) true true "(R=0.000000,G=0.660000,B=1.000000,A=1.000000)" 5.0)
  ;[1 1 1] Move Player Forward one Crossing
  (Variables|Default|SetPositionOnMap (Variables|/Game/Escape_Van/Blueprints/Crossing.Crossing_C|GetCoordinates (Variables|Default|GetNextCrossing)))
  (bind (_nextcrossingcoords _nextcrossing _success) (CallFunction|FindNextCrossing))
  (Variables|Default|SetNextCrossing _nextcrossing)
  (Development|PrintString (Utilities|String|Append "Next Crossing at: " (Utilities|String|ToString(Vector2d) _nextcrossingcoords)) true true "(R=0.000000,G=0.660000,B=1.000000,A=1.000000)" 1e+01)
  (if _success
    (Default|StartNewRound (Variables|References|GetGameMode))))

(event EventBeginPlay
  (bind _asgm_escape_van_alpha_1 (Utilities|Casting|CastToGM_Escape_Van_Alpha1 (Game|GetGameMode))
    (:then
      (Variables|References|SetGameMode _asgm_escape_van_alpha_1)
      (bind _aspawn_van (Utilities|Casting|CastToPawn_Van (Game|Player|GetPlayerPawn 0))
        (:then
          (Variables|Default|SetPlayerPawn _aspawn_van)
          (bind _nextcrossing (CallFunction|FindNextCrossing))
          (Variables|Default|SetNextCrossing _nextcrossing)
          (Default|StartNewRound (Variables|References|GetGameMode)))
        (:CastFailed
          (Development|PrintString "Cast Failed" :!label _label))))
    (:CastFailed
      (goto _label))))

(event Input|KeyboardEvents|SpaceBar
  (params (Key :type Key%20Structure :default "None"))
  (bind _positiononmap (Variables|Default|GetPositionOnMap))
  (bind _heading (Variables|Default|GetHeading))
  (bind _gamemode (Variables|References|GetGameMode))
  (bind _returnvalue (Class|KismetMathLibrary|GetRotated2D _heading -9e+01))
  (bind _crossing_coords (Variables|/Game/Escape_Van/Core/GM_Escape_Van_Alpha1.GM_Escape_Van_Alpha1_C|GetCrossing_Coords _gamemode))
  (bind _returnvalue_2 (Class|KismetMathLibrary|ToIntPoint(Vector2D) _returnvalue))
  (bind _returnvalue_3 (Math|Conversions|ToVector2D(IntPoint) _returnvalue_2))
  (bind _returnvalue_4 (+ _positiononmap _returnvalue_3))
  (:Pressed
    (Development|PrintString (Utilities|String|Append "Checking for" (Utilities|String|ToString(Vector2d) _returnvalue_4)))
    (bind _keys (Utilities|Map|Keys _crossing_coords))
    (if (Utilities|Map|Contains _crossing_coords _returnvalue_4)
      (Development|PrintString "True"))))

(fn ConstructionScript)

(fn FindNextCrossing
  (bind _gamemode (Variables|References|GetGameMode))
  (bind _positiononmap (Variables|Default|GetPositionOnMap))
  (bind _heading (Variables|Default|GetHeading))
  (bind _returnvalue (+ _positiononmap _heading))
  (bind _crossing_coords (Variables|/Game/Escape_Van/Core/GM_Escape_Van_Alpha1.GM_Escape_Van_Alpha1_C|GetCrossing_Coords _gamemode))
  (bind (_value _returnvalue_2) (Utilities|Map|Find _crossing_coords _returnvalue))
  (bind _returnvalue_3 (Utilities|String|ToString(Vector2d) _returnvalue))
  (Development|PrintString (Utilities|String|Append "Searching for: " _returnvalue_3) true true "(R=0.000000,G=0.660000,B=1.000000,A=1.000000)" 1e+01)
  (if _returnvalue_2
    (Development|PrintString "Found" true true "(R=0.000000,G=0.660000,B=1.000000,A=1.000000)" 1e+01)
    (return _returnvalue _value _returnvalue_2)
    (else
      (Development|PrintString (Utilities|String|Append _returnvalue_3 " was not found") true true "(R=0.000000,G=0.660000,B=1.000000,A=1.000000)" 1e+01))))